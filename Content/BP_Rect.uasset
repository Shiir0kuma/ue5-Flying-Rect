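; BP_Rect is a player-controlled pawn Blueprint driven by Enhanced Input.
; BeginPlay adds the IMC_Rect mapping context to player controller 0.
; IA_Move feeds forward movement from its Y axis and turns the actor in local yaw from its X axis, tank-style, while IA_UpDown moves it along its up vector.
; Yaw is applied per input event without delta-time scaling.
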(event `EnhancedInput|/Game/IA_UpDown`
  (params (ActionValue :type "Float (double-precision)") (ElapsedSeconds :type "Float (double-precision)") (TriggeredSeconds :type "Float (double-precision)") (InputAction :type "InputAction Object Reference" :default "/Game/IA_UpDown.IA_UpDown"))
  (:`Triggered`
    (`self.AddMovementInput` (`self.GetActorUpVector`) ActionValue)))

(event `EnhancedInput|/Game/IA_Move`
  (params (ActionValue :type "Vector2D Structure") (ElapsedSeconds :type "Float (double-precision)") (TriggeredSeconds :type "Float (double-precision)") (InputAction :type "InputAction Object Reference" :default "/Game/IA_Move.IA_Move"))
  (bind (_x _y) (`KismetMathLibrary.BreakVector2D` ActionValue))
  (:`Triggered`
    (`self.AddMovementInput` (`self.GetActorForwardVector`) _y)
    (`self.K2_AddActorLocalRotation` (`KismetMathLibrary.MakeRotator` 0.0 0.0 (* _x 2.0)))))

(event `self.ReceiveBeginPlay`
  (`EnhancedInputSubsystemInterface.AddMappingContext` (pcsubsystem `EnhancedInputLocalPlayerSubsystem` (`GameplayStatics.GetPlayerController` 0)) "/Game/IMC_Rect.IMC_Rect" 0 (struct)))

(fn `UserConstructionScript`)